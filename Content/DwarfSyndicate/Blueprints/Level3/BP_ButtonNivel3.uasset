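; A puzzle button actor for Level 3 that registers its key with the Level3Manager when pressed through interaction.
; It finds the manager on BeginPlay, starts with its light off, and only submits on the first press via a Pressed flag.
; Correct and Wrong events light it green persistently or flash it red for a second, with debug prints; this Blueprint never resets Pressed.
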(event `self.ReceiveBeginPlay`
  (`parent.ReceiveBeginPlay`)
  (bind _returnvalue (`GameplayStatics.GetActorOfClass` "/Game/DwarfSyndicate/Blueprints/Level3/Level3Manager.Level3Manager_C"))
  (set `self.LevelManagerRef` _returnvalue)
  (`LightComponent.SetIntensity` (`self.light`) 0.0))

(event `Press`
  (if (not (`self.pressed`))
    (set `self.pressed` true)
    (`/Game/DwarfSyndicate/Blueprints/Level3/Level3Manager.AddButton` (`self.LevelManagerRef`) (`self.Key`))))

(event `Correct`
  (bind _light (`self.light`))
  (`LightComponent.SetIntensity` _light (`self.intensityLight`))
  (`LightComponent.SetLightColor` _light (struct :`R` 0.071829 :`G` 1.0 :`B` 0.123349 :`A` 1.0) true)
  (`KismetSystemLibrary.PrintText` "correct"))

(event `Wrong`
  (bind _light (`self.light`))
  (`LightComponent.SetIntensity` _light (`self.intensityLight`))
  (`LightComponent.SetLightColor` _light (struct :`R` 1.0 :`B` 0.0848 :`A` 1.0) true)
  (`KismetSystemLibrary.Delay` 1.0)
  (`LightComponent.SetIntensity` (`self.light`) 0.0)
  (`KismetSystemLibrary.PrintText` "wrong"))

(event `/Game/DwarfSyndicate/Blueprints/Puzzles/BI_Interactables.OnInteraction`
  (`self.Press`)
  (`KismetSystemLibrary.PrintText` "pressed"))

(fn `UserConstructionScript`
  (`parent.UserConstructionScript`))
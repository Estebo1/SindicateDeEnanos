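; Level 3 manager for an ordered button puzzle that reveals the level's pressure plate when solved.
; AddButton records each key until solved, and CheckAnswer re-compares all entries with CorrectAnswer, marking Buttons by entry position.
; A mismatch resets every button and clears the input.
; Solved is called inside the compare loop once five keys are entered, so it can fire before later entries are checked.
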(event `self.ReceiveBeginPlay`)

(event `AddButton`
  (params (Key :type Integer))
  (if (not (`self.solvedPuzzle`))
    (`KismetArrayLibrary.Array_Add` (`self.EnteringAnswers`) Key)
    (set `self.currentIndex` (+ (`self.currentIndex`) 1))
    (`self.CheckAnswer`)))

(event `CheckAnswer`
  (for _index (range (`self.currentIndex`))
    (if (== (`|GetArrayItem` (`self.CorrectAnswer`) _index) (`|GetArrayItem` (`self.EnteringAnswers`) _index))
      (`/Game/DwarfSyndicate/Blueprints/Level3/BP_ButtonNivel3.Correct` (`|GetArrayItem` (`self.buttons`) _index))
      (if (== (`self.currentIndex`) 5)
        (`self.Solved`))
      (else
        (set `self.solvedPuzzle` false)
        (`self.ResetButtons`)
        (break)))))

(event `Solved`
  (set `self.solvedPuzzle` true)
  (bind _returnvalue (`GameplayStatics.GetActorOfClass` "/Game/DwarfSyndicate/Blueprints/Level3/BP_Level3PressurePlate.BP_Level3PressurePlate_C"))
  (`/Game/DwarfSyndicate/Blueprints/Level3/BP_Level3PressurePlate.Visibile` _returnvalue))

(event `ResetButtons`
  (set `self.currentIndex` 0)
  (for _array_element (`self.buttons`)
    (set `/Game/DwarfSyndicate/Blueprints/Level3/BP_ButtonNivel3.pressed` false _array_element)
    (`/Game/DwarfSyndicate/Blueprints/Level3/BP_ButtonNivel3.Wrong` _array_element))
  (`KismetArrayLibrary.Array_Clear` (`self.EnteringAnswers`)))

(fn `UserConstructionScript`)
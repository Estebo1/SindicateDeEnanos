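; Level 3 pressure plate that opens the level's BP_DoorLevel3 when the dwarf or the orc (BP_ThirdPersonCharacter) steps on it.
; Box overlaps set a flag per character and call the door, found at BeginPlay along with an otherwise unused Level3Manager.
; CheckBox closes the door unless both flags remain set, so either character leaving closes it.
; Visibile and Invisible events toggle the sphere's visibility and the box's query collision.
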(event `self.ReceiveBeginPlay`
  (bind _returnvalue (`GameplayStatics.GetActorOfClass` "/Game/DwarfSyndicate/Blueprints/Level3/Level3Manager.Level3Manager_C"))
  (set `self.levelManager` _returnvalue)
  (bind _returnvalue_2 (`GameplayStatics.GetActorOfClass` "/Game/DwarfSyndicate/Blueprints/Level3/BP_DoorLevel3.BP_DoorLevel3_C"))
  (set `self.DoorRef` _returnvalue_2))

(event `Invisible`
  (`SceneComponent.SetVisibility` (`self.Sphere`) false false)
  (`PrimitiveComponent.SetCollisionEnabled` (`self.Box`) "NoCollision"))

(event `Visibile`
  (`SceneComponent.SetVisibility` (`self.Sphere`) true false)
  (`PrimitiveComponent.SetCollisionEnabled` (`self.Box`) "QueryOnly"))

(event `self.Box.OnComponentBeginOverlap`
  (params (OverlappedComponent :type "PrimitiveComponent Object Reference") (OtherActor :type "Actor Object Reference") (OtherComp :type "PrimitiveComponent Object Reference") (OtherBodyIndex :type Integer) (bFromSweep :type Boolean) (SweepResult :type "HitResult Structure (by ref)"))
  (if (`GameplayStatics.ObjectIsA` OtherActor "/Game/DwarfSyndicate/Blueprints/BP_Dwarf.BP_Dwarf_C")
    (set `self.DwarfIsOn` true)
    (`self.Activate` :!label _label)
    (elif (`GameplayStatics.ObjectIsA` OtherActor "/Game/DwarfSyndicate/Blueprints/BP_ThirdPersonCharacter.BP_ThirdPersonCharacter_C")
      (set `self.OrcfIsOn` true)
      (goto _label))))

(event `self.Box.OnComponentEndOverlap`
  (params (OverlappedComponent :type "PrimitiveComponent Object Reference") (OtherActor :type "Actor Object Reference") (OtherComp :type "PrimitiveComponent Object Reference") (OtherBodyIndex :type Integer))
  (if (`GameplayStatics.ObjectIsA` OtherActor "/Game/DwarfSyndicate/Blueprints/BP_Dwarf.BP_Dwarf_C")
    (set `self.DwarfIsOn` false)
    (`self.CheckBox` :!label _label_2)
    (elif (`GameplayStatics.ObjectIsA` OtherActor "/Game/DwarfSyndicate/Blueprints/BP_ThirdPersonCharacter.BP_ThirdPersonCharacter_C")
      (set `self.OrcfIsOn` false)
      (goto _label_2))))

(event `CheckBox`
  (if (not (and (`self.DwarfIsOn`) (`self.OrcfIsOn`)))
    (`self.Deactivate`)))

(event `Activate`
  (`/Game/DwarfSyndicate/Blueprints/Level3/BP_DoorLevel3.OpenDoor` (`self.DoorRef`) true))

(event `Deactivate`
  (`/Game/DwarfSyndicate/Blueprints/Level3/BP_DoorLevel3.OpenDoor` (`self.DoorRef`) false))

(fn `UserConstructionScript`)
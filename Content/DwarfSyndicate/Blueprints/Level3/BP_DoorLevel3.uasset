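; BP_DoorLevel3 is a Level 3 door that moves vertically between its starting position and a raised or lowered position.
; On BeginPlay it caches its location and builds an end point at the same X and Y, using DoorHeight as an absolute world Z.
; The OpenDoor event plays or reverses the MoveDoor timeline from its IsActivated flag, lerping the actor between the two points without sweep.
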(event `self.ReceiveBeginPlay`
  (bind _output_get (set `self.StartLocation` (`self.K2_GetActorLocation`)))
  (set `self.EndLocation` (`KismetMathLibrary.MakeVector` (.x _output_get) (.y _output_get) (`self.doorHeight`))))

(event `OpenDoor`
  (params (isActivated :type Boolean))
  (if isActivated
    (bind (_direction _float) (`Timeline|MoveDoor` :!label _label)
      (:`Update`
        (`self.K2_SetActorLocation` (`KismetMathLibrary.VLerp` (`self.StartLocation`) (`self.EndLocation`) _float))))
    (else
      (goto _label :!via `Reverse`))))

(fn `UserConstructionScript`)
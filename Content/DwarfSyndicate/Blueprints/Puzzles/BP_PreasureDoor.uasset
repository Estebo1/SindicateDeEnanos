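; Puzzle-driven door, named as a pressure door, that slides vertically when its puzzle is solved or unsolved.
; SolvePuzzle reverses a timeline and UnsolvePuzzle plays it forward, with its Angle track lerping the Pivot's relative height between raised and lowered positions.
; IsClosed toggles whenever the timeline finishes, while OnInteraction is left empty.
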(event `/Game/DwarfSyndicate/Blueprints/Puzzles/BI_Interactables.OnInteraction`)

(event `/Game/DwarfSyndicate/Blueprints/Puzzles/BP_PuzzleProblem.SolvePuzzle`
  (bind _pivot (`self.Pivot`))
  (bind (_relativelocation_x _relativelocation_y) (`KismetMathLibrary.BreakVector` (`SceneComponent.RelativeLocation` _pivot)))
  (bind (_direction _angle) (`Timeline|Timeline` :!via `Reverse` :!label _label)
    (:`Update`
      (`SceneComponent.K2_SetRelativeLocation` _pivot (`KismetMathLibrary.MakeVector` _relativelocation_x _relativelocation_y (`KismetMathLibrary.Lerp` 200.0 1.0 _angle)) false false))
    (:`Finished`
      (set `self.isClosed` (not (`self.isClosed`))))))

(event `/Game/DwarfSyndicate/Blueprints/Puzzles/BP_PuzzleProblem.UnsolvePuzzle`
  (goto _label))

(fn `UserConstructionScript`
  (`parent.UserConstructionScript`))
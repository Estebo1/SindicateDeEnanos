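; BP_Key is a collectible puzzle key actor that spins in the world until interacted with.
; Tick sets the Key component's world yaw from CurRot, which adds delta time and then multiplies the whole sum by SpeedRotation, so it compounds each frame.
; OnInteraction checks that MyPuzzleProblem is valid, calls SolvePuzzle on it, prints a Spanish collected message and destroys the key.
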(event `self.ReceiveTick`
  (params (DeltaSeconds :type "Float (single-precision)"))
  (bind _output_get (set `self.curRot` (* (+ DeltaSeconds (`self.curRot`)) (`self.speed rotation`))))
  (`SceneComponent.K2_SetWorldRotation` (`self.key`) (`KismetMathLibrary.MakeRotator` 0.0 0.0 _output_get) false false))

(event `/Game/DwarfSyndicate/Blueprints/Puzzles/BI_Interactables.OnInteraction`
  (bind _mypuzzleproblem (`self.MyPuzzleProblem`)
    (:`then`
      (`/Game/DwarfSyndicate/Blueprints/Puzzles/BP_PuzzleProblem.SolvePuzzle` _mypuzzleproblem)
      (`KismetSystemLibrary.PrintText` "Se recolectó ")
      (`self.K2_DestroyActor`))
    (:`else`)))

(fn `UserConstructionScript`
  (`parent.UserConstructionScript`))
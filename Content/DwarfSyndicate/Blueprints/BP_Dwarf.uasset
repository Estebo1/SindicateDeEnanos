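; BP_Dwarf is an NPC dwarf that can be toggled to follow the player through interaction.
; While following, PawnSensing sightings issue AI move orders toward the seen pawn, and a follow indicator widget reflects the current state.
; An overlap collider shows and hides a message widget when the player character enters or leaves.
; Every tick it rotates to face the cached player reference, re-fetching that reference if invalid.
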(event `self.ReceiveBeginPlay`
  (`SceneComponent.SetVisibility` (`self.Widget`) false false)
  (bind _aswdg_follow_indicator (cast `/Game/DwarfSyndicate/Widgets/WDG_FollowIndicator` (`WidgetComponent.GetWidget` (`self.FollowWidget`))))
  (`/Game/DwarfSyndicate/Widgets/WDG_FollowIndicator.UpdateFollowIcon` _aswdg_follow_indicator false)
  (`self.GetAnimationBp`)
  (`self.GetPlayerRef`))

(event `self.PawnSensing.OnSeePawn`
  (params (Pawn :type "Pawn Object Reference"))
  (if (`self.Follow`)
    (`|AIMoveTo` self (0.0 0.0 0.0) Pawn 150.0)))

(event `/Game/DwarfSyndicate/Blueprints/Puzzles/BI_Interactables.OnInteraction`
  (bind _output_get (set `self.Follow` (not (`self.Follow`))))
  (bind _aswdg_follow_indicator (cast `/Game/DwarfSyndicate/Widgets/WDG_FollowIndicator` (`WidgetComponent.GetWidget` (`self.FollowWidget`))))
  (`/Game/DwarfSyndicate/Widgets/WDG_FollowIndicator.UpdateFollowIcon` _aswdg_follow_indicator _output_get))

(event `self.MessageCol.OnComponentBeginOverlap`
  (params (OverlappedComponent :type "PrimitiveComponent Object Reference") (OtherActor :type "Actor Object Reference") (OtherComp :type "PrimitiveComponent Object Reference") (OtherBodyIndex :type Integer) (bFromSweep :type Boolean) (SweepResult :type "HitResult Structure (by ref)"))
  (cast `/Game/DwarfSyndicate/Blueprints/BP_ThirdPersonCharacter` OtherActor)
  (`SceneComponent.SetVisibility` (`self.Widget`) true false))

(event `GetPlayerRef`
  (bind _returnvalue (`GameplayStatics.GetActorOfClass` "/Game/DwarfSyndicate/Blueprints/BP_ThirdPersonCharacter.BP_ThirdPersonCharacter_C"))
  (set `self.playerRef` _returnvalue))

(event `self.MessageCol.OnComponentEndOverlap`
  (params (OverlappedComponent :type "PrimitiveComponent Object Reference") (OtherActor :type "Actor Object Reference") (OtherComp :type "PrimitiveComponent Object Reference") (OtherBodyIndex :type Integer))
  (cast `/Game/DwarfSyndicate/Blueprints/BP_ThirdPersonCharacter` OtherActor)
  (`SceneComponent.SetVisibility` (`self.Widget`) false false))

(event `self.ReceiveTick`
  (params (DeltaSeconds :type "Float (single-precision)"))
  (bind _playerref (`self.playerRef`))
  (`/Engine/EditorBlueprintResources/StandardMacros.IsValid` _playerref
    (:`Is Valid`
      _)
    (:`Is Not Valid`
      (`self.GetPlayerRef`)))
  (`self.K2_SetActorRotation` self (`KismetMathLibrary.FindLookAtRotation` (`self.K2_GetActorLocation` self) (`self.K2_GetActorLocation` _playerref)) false))

(fn `GetAnimationBp`
  (bind _asabp_dwarf (cast `/Game/DwarfSyndicate/Animation/Dwarf/ABP_Dwarf` (`SkeletalMeshComponent.GetAnimInstance` (`self.Mesh`))))
  (set `self.abpDwarf` _asabp_dwarf))

(fn `UserConstructionScript`)